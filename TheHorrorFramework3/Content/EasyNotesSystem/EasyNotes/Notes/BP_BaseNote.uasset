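; Base actor for a readable note that the player interacts with through an interface, which also reports whether it can be interacted with.
; Interacting creates a WB_Notes widget from NoteData, shows it with the cursor in UI-only input, or prints an error if the data is missing.
; When DestroyAfterRead is set, Tick polls for the widget leaving the viewport, then plays a take sound once and destroys the note.
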(event EventBPIInteract
  ;[0.4508 0.3005 1] Interact funtion | Open Widget, Set Input Mode Ui Only
  (bind _notedata (Variables|NoteSettings|GetNoteData)
    (:then
      (bind _returnvalue (UserInterface|CreateWidget "/Game/EasyNotesSystem/EasyNotes/Core/Widgets/WB_Notes.WB_Notes_C" 0 _notedata))
      (bind _output_get (Variables|References|SetNoteWidget _returnvalue))
      (Variables|Variables|SetIsInViewport? true)
      (UserInterface|Viewport|AddtoViewport _output_get 0)
      (Input|SetInputModeUIOnly (Game|GetPlayerController 0) 0 "DoNotLock" false)
      (Variables|/Script/Engine.PlayerController|SetbShowMouseCursor (Game|GetPlayerController 0) true))
    (:else
      (Development|PrintString "NoteData not set!"))))

(event EventTick
  (params (DeltaSeconds :type Float%20%28single-precision%29))
  ;[0.4488 0.3015 1] Event Tick
  (CallFunction|DestroyAfterRead (Variables|NoteSettings|GetDestroyAfterRead?)))

(fn ConstructionScript)

(fn DestroyAfterRead
  (params (Destroy? :type Boolean))
  (if Destroy?
    (if (Variables|Variables|GetIsInViewport?)
      (if (not (UserInterface|Viewport|IsinViewport (Variables|References|GetNoteWidget)))
        (Utilities|FlowControl|DoOnce false
          (:Completed
            (Audio|PlaySoundatLocation "/Game/EasyNotesSystem/EasyNotes/Core/Widgets/Assets/Sounds/SW_Note_Take_Note.SW_Note_Take_Note" (Transformation|GetActorLocation) "0, 0, 0" 1.0 1.0 0.0 "/Game/EasyNotesSystem/EasyNotes/Core/Widgets/Assets/Sounds/SA_Note.SA_Note" 0 0 0)
            (Actor|DestroyActor)))))))

(fn BPICanInteract?
  (return (Variables|Variables|GetCanInteract?)))