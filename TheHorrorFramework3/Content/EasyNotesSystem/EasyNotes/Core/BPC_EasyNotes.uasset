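; BPC_EasyNotes is a component of the Easy Notes system that lets the player interact with actors in view.
; Each tick, it line-traces a short distance from the camera on Visibility, with debug drawing, caching the hit actor and its BPI_Interactable can-interact result.
; Pressing E sends the interact message to that actor if allowed.
; A trace miss leaves the cached values intact, so the last target remains usable.
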(event EventTick
  (params (DeltaSeconds :type Float%20%28single-precision%29))
  ;[0.4488 0.3015 1] Event Tick | Interaction Line Trace
  (Interaction|InteractionLineTrace 2e+02 "ForOneFrame"))

(event Input|KeyboardEvents|E
  (params (Key :type Key%20Structure :default "None"))
  ;[0.4471 0.302 1] Interaction Input
  (:Pressed
    (Interaction|Interact)))

(fn InteractionLineTrace
  (params (TraceDistance :type Float%20%28single-precision%29) (DrawDebugType :type EDrawDebugTrace%20Enum :default "None"))
  (bind _returnvalue (Game|GetPlayerCameraManager 0))
  (bind _transformcomponent (Variables|/Script/Engine.PlayerCameraManager|GetTransformComponent _returnvalue))
  (bind _returnvalue_2 (Transformation|GetWorldLocation _transformcomponent))
  (bind (_outhit _returnvalue_3) (Collision|LineTraceByChannel _returnvalue_2 (+ _returnvalue_2 (* (Math|Vector|GetForwardVector _transformcomponent) TraceDistance)) "TraceTypeQuery1" false 0 DrawDebugType true "(R=0.447059,G=0.301961,B=1.000000,A=1.000000)"))
  (if _returnvalue_3
    (bind _output_get (Variables|References|InteractionLineTrace|SetHitActor (.HitActor (Collision|BreakHitResult _outhit))))
    (if (Utilities|DoesObjectImplementInterface _output_get "/Game/EasyNotesSystem/EasyNotes/Core/DataTypes/Interface/BPI_Interactable.BPI_Interactable_C")
      (bind _caninteract_ (Class|BPIInteractable|BPICanInteract?(Message) (Variables|References|InteractionLineTrace|GetHitActor)))
      (Variables|InteractionTrace|SetCanInteract? _caninteract_)
      (else
        (Variables|InteractionTrace|SetCanInteract? false)))))

(fn Interact
  (if (Variables|InteractionTrace|GetCanInteract?)
    (Class|BPIInteractable|BPIInteract(Message) (Variables|References|InteractionLineTrace|GetHitActor))))